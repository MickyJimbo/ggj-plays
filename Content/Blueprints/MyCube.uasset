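; MyCube is a cube actor that the player nudges left and right along Y with the arrow keys.
; BeginPlay enables input for player 0 and adds a HUD widget to the viewport.
; Key presses call Move, which recolors the cube blue or green and offsets it by AmountOfMovement divided by Players, feeding world coordinates into SetRelativeLocation.
; An edge check that would enable physics is left unconnected.
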(event EventBeginPlay
  (Utilities|FlowControl|Sequence
    (:then_0
      (Input|EnableInput (Game|GetPlayerController 0)))
    (:then_1
      (bind _returnvalue (UserInterface|CreateWidget "/Game/Blueprints/HUD.HUD_C"))
      (UserInterface|Viewport|AddtoViewport _returnvalue 0))))

(event EventTick
  (params (DeltaSeconds :type Float%20%28single-precision%29)))

(event Input|KeyboardEvents|Left
  (params (Key :type Key%20Structure))
  ;[1 1 1] Movment
  (:Pressed
    (Development|PrintString "left")
    (CallFunction|Move "NewEnumerator0" 1)))

(event Input|KeyboardEvents|Right
  (params (Key :type Key%20Structure))
  ;[1 1 1] Movment
  (:Pressed
    (Development|PrintString "right")
    (CallFunction|Move "NewEnumerator1" 1)))

(fn ConstructionScript)

(fn Move
  (params (Side :type SideEnum%20Enum :default "NewEnumerator0") (Players :type Integer))
  (bind _returnvalue (Math|Conversions|ToFloat(Integer) Players))
  (bind _amountofmovement (Variables|Default|GetamountOfMovement))
  (bind _cube (Variables|Default|GetCube))
  (bind _cube_2 (Variables|Default|GetCube))
  (bind _cube_3 (Variables|Default|GetCube))
  (bind _cube_4 (Variables|Default|GetCube))
  (bind _returnvalue_2 (/ _amountofmovement _returnvalue))
  (bind _returnvalue_3 (Transformation|GetWorldLocation _cube))
  (bind _returnvalue_4 (Transformation|GetWorldLocation _cube_2))
  (bind (_x _y _z) (Math|Vector|BreakVector _returnvalue_3))
  (bind (_x_2 _y_2 _z_2) (Math|Vector|BreakVector _returnvalue_4))
  (switch Utilities|FlowControl|Switch|SwitchonSideEnum Side
    (:NewEnumerator0
      (Rendering|Material|SetMaterial _cube_4 0 "/Game/Materials/TronGlow_Blue.TronGlow_Blue")
      (Transformation|SetRelativeLocation _cube_4 (Math|Vector|MakeVector _x_2 (- _y_2 _returnvalue_2) _z_2) false false))
    (:NewEnumerator1
      (Rendering|Material|SetMaterial _cube_3 0 "/Game/Materials/TronGlow_Green.TronGlow_Green")
      (Transformation|SetRelativeLocation _cube_3 (Math|Vector|MakeVector _x (+ _y _returnvalue_2) _z) false false))))