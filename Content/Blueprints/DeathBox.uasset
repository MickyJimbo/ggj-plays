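; DeathBox is a kill volume that ends the game when the player's cube falls into or touches it.
; On overlap with MyCube it flags the loss, stops the GameManager's background music, plays the Lose sound and reloads the Game level after a short delay.
; Any other overlapping actor is destroyed.
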(event Collision|EventActorBeginOverlap
  (params (OtherActor :type Actor%20Object%20Reference))
  (bind _asmy_cube (Utilities|Casting|CastToMyCube OtherActor)
    (:then
      (Variables|/Game/Blueprints/MyCube.MyCube_C|SethasLost _asmy_cube true)
      (bind _outactors (Actor|GetAllActorsOfClass "/Game/Blueprints/GameManager.GameManager_C"))
      (bind _asgame_manager (Utilities|Casting|CastToGameManager (Utilities|Array|Get(acopy) _outactors)))
      (Audio|Components|Audio|Stop (Variables|/Game/Blueprints/GameManager.GameManager_C|Getbgm _asgame_manager))
      (Audio|Components|Audio|Play (Variables|Default|GetLose) 0.0)
      (Utilities|FlowControl|Delay 2.0)
      (Game|OpenLevel(byName) "Game"))
    (:CastFailed
      (Actor|DestroyActor OtherActor))))

(fn ConstructionScript)