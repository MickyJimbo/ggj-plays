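; Wall is an obstacle actor that can move and awards a point when the MyCube passes into its success trigger.
; A timeline offsets it from its initial location while CanMove is set, and the construction script picks a random mesh from WallMeshes.
; The trigger uses DoOnce to increment the GameManager's Score and play a ping.
; Hits from the cube play a thud.
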(event OnComponentBeginOverlap(SuccessTrigger)
  (params (OverlappedComponent :type Primitive%20Component%20Object%20Reference) (OtherActor :type Actor%20Object%20Reference) (OtherComp :type Primitive%20Component%20Object%20Reference) (OtherBodyIndex :type Integer) (bFromSweep :type Boolean) (SweepResult :type Hit%20Result%20Structure%20%28by%20ref%29))
  ;[1 1 1] On Success Trigger
  (Utilities|Casting|CastToMyCube OtherActor)
  (Utilities|FlowControl|DoOnce false
    (:Completed
      (Utilities|FlowControl|Sequence
        (:then_1
          (bind _outactors (Actor|GetAllActorsOfClass "/Game/Blueprints/GameManager.GameManager_C"))
          (Variables|/Game/Blueprints/GameManager.GameManager_C|Setscore (Utilities|Array|Get(acopy) _outactors) (+ (Variables|/Game/Blueprints/GameManager.GameManager_C|Getscore (Utilities|Array|Get(acopy) _outactors)) 1))
          (Audio|Components|Audio|Play (Variables|Default|Getping) 0.0))))))

(event OnComponentHit(Wall)
  (params (HitComponent :type Primitive%20Component%20Object%20Reference) (OtherActor :type Actor%20Object%20Reference) (OtherComp :type Primitive%20Component%20Object%20Reference) (NormalImpulse :type Vector :default "0, 0, 0") (Hit :type Hit%20Result%20Structure%20%28by%20ref%29))
  (Utilities|Casting|CastToMyCube OtherActor)
  (Audio|Components|Audio|Play (Variables|Default|GetThud) 0.0))

(event EventBeginPlay
  ;[1 1 1] Begin play
  (Variables|Default|SetInitial_location (Transformation|GetActorLocation))
  (bind _movement (Timeline|Timeline_0 PlayFromStart)
    (:Update
      (if (Variables|Default|GetcanMove)
        (Transformation|SetActorLocation (+ (Variables|Default|GetInitial_location) _movement) false false)))))

(fn ConstructionScript
  (bind _wall_meshes (Variables|Default|GetWall_Meshes))
  (Components|StaticMesh|SetStaticMesh (Variables|Default|GetWall) (Utilities|Array|Get(acopy) _wall_meshes (Math|Random|RandomIntegerinRange 0 (- (Utilities|Array|Length _wall_meshes) 1)))))