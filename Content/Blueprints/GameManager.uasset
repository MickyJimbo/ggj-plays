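; GameManager connects to a TCP server and turns received messages into left or right moves of a MyCube actor.
; On BeginPlay it relocates the player pawn, spawns a Wall, binds the TCP client's connect and message events, and caches all MyCube actors.
; Quoted "left" or "right" messages call Move on the first cube with the stored player count; any other message is parsed as that count.
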(event Custom|Connecting
  (params (Connected :type Boolean))
  (if Connected
    (Development|PrintString "Connected")))

(event Custom|NewMessage
  (params (Message :type String))
  (if (Utilities|Enum|Equal(Enum) Message "\"left\"")
    (Default|Move (Utilities|Array|Get(acopy) (stale EventBeginPlay _outactors)) "NewEnumerator0" (Variables|Default|GetnumberOfPlayers))
    (elif (Utilities|Enum|Equal(Enum) Message "\"right\"")
      (Default|Move (Utilities|Array|Get(acopy) (stale EventBeginPlay _outactors)) "NewEnumerator1" (Variables|Default|GetnumberOfPlayers))
      (else
        (Variables|Default|SetnumberOfPlayers (Math|Conversions|ToInteger(Byte) Message))))))

(event EventBeginPlay
  (bind _tcpclient (Variables|Default|GetTCPClient))
  (Utilities|FlowControl|Sequence
    (:then_0
      (Transformation|SetActorRelativeLocation (Game|Player|GetPlayerPawn 0) "5000.000000,5000.000000,5000.000000"))
    (:then_1
      (Game|SpawnActorfromClass "/Game/Blueprints/Wall.Wall_C" (Math|Conversions|ToTransform(Vector) "1000.000000,0.000000,20.000000") "Undefined" 0 0))
    (:then_2
      (EventDispatchers|BindEventtoOnConnect _tcpclient (delegate Custom|Connecting))
      (Class|TCPClient|Connect _tcpclient)
      (EventDispatchers|BindEventtoOnMessage _tcpclient (delegate Custom|NewMessage))
      (bind _outactors (Actor|GetAllActorsOfClass "/Game/Blueprints/MyCube.MyCube_C")))))

(event Collision|EventActorBeginOverlap
  (params (OtherActor :type Actor%20Object%20Reference)))

(event EventTick
  (params (DeltaSeconds :type Float%20%28single-precision%29)))

(fn ConstructionScript)